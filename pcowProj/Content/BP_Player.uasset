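; Player actor that moves with input and collects bananas, shifting its cube's color as the count grows.
; The MoveRight axis drives a swept, frame-time-scaled world offset on both X and Y; MoveForward has no logic.
; Mesh overlaps with Banana_Blueprint destroy the banana and increment a counter.
; The counter, normalized and clamped, sets the ColorAlpha parameter on a dynamic material created at BeginPlay.
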(event OnComponentBeginOverlap(StaticMesh)
  (params (OverlappedComponent :type Primitive%20Component%20Object%20Reference) (OtherActor :type Actor%20Object%20Reference) (OtherComp :type Primitive%20Component%20Object%20Reference) (OtherBodyIndex :type Integer) (bFromSweep :type Boolean) (SweepResult :type Hit%20Result%20Structure%20%28by%20ref%29))
  (bind _asbanana_blueprint (Utilities|Casting|CastToBanana_Blueprint OtherActor))
  (bind _result (Math|Float|IncrementFloat (Variables|Default|GetBananaCounter))
    (:%20%20
      (Actor|DestroyActor _asbanana_blueprint)
      (Rendering|Material|SetScalarParameterValue (Variables|Default|GetCubeMaterial) "ColorAlpha" (Math|Float|Clamp(Float) (/ _result 18.0)) :!class /Script/Engine.MaterialInstanceDynamic))))

(event EventBeginPlay
  (bind _returnvalue (Rendering|Material|CreateDynamicMaterialInstance (Variables|Default|GetStaticMesh) 0 "/Game/Materials/M_Cube.M_Cube" "None" :!class /Script/Engine.PrimitiveComponent))
  (Variables|Default|SetCubeMaterial _returnvalue))

(event EventTick
  (params (DeltaSeconds :type Float%20%28single-precision%29)))

(event Input|AxisEvents|InputAxisMoveRight
  (params (AxisValue :type Float%20%28single-precision%29))
  (Transformation|AddActorWorldOffset (Math|Vector|MakeVector (* (stale Input|AxisEvents|InputAxisMoveForward AxisValue) (Variables|Default|GetspeedForward) (stale EventTick DeltaSeconds)) (* AxisValue (Variables|Default|GetspeedRight) (stale EventTick DeltaSeconds)) 0.0) true))

(event Input|AxisEvents|InputAxisMoveForward
  (params (AxisValue :type Float%20%28single-precision%29)))

(fn ConstructionScript)