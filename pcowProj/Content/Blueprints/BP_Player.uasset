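; Player actor that moves through the level collecting bananas on overlap.
; The MoveRight axis drives a swept, delta-time-scaled world offset in X and Y, while MoveForward is empty.
; BeginPlay creates the HUD, a dynamic cube material and stores the BP_GenerateBananas starting count.
; Each pickup destroys the banana, raises the ColorAlpha material parameter by collected fraction, decrements the generator's count and refreshes the HUD.
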(event OnComponentBeginOverlap(StaticMesh)
  (params (OverlappedComponent :type Primitive%20Component%20Object%20Reference) (OtherActor :type Actor%20Object%20Reference) (OtherComp :type Primitive%20Component%20Object%20Reference) (OtherBodyIndex :type Integer) (bFromSweep :type Boolean) (SweepResult :type Hit%20Result%20Structure%20%28by%20ref%29))
  (bind _asbp_banana (Utilities|Casting|CastToBP_Banana OtherActor))
  (Utilities|FlowControl|Sequence
    (:then_0
      (bind _result (Math|Float|IncrementFloat (Variables|Default|GetBananaCounter))
        (:%20%20
          (Actor|DestroyActor _asbp_banana))))
    (:then_1
      (Rendering|Material|SetScalarParameterValue (Variables|Default|GetCubeMaterial) "ColorAlpha" (Math|Float|Clamp(Float) (/ _result (Math|Conversions|ToFloat(Integer) (Variables|Default|GetBananaFirstCount)))) :!class /Script/Engine.MaterialInstanceDynamic))
    (:then_2
      (Math|Integer|DecrementInt (Variables|/Game/Blueprints/BP_GenerateBananas.BP_GenerateBananas_C|GetCount (Variables|Default|GetBananaGenerator))
        (:%20%20
          (Default|UpdateCounterText (Variables|Default|GetHUD)))))))

(event EventBeginPlay
  (Utilities|FlowControl|Sequence
    (:then_0
      (bind _returnvalue (UserInterface|CreateWidget "/Game/UI/HUD.HUD_C"))
      (UserInterface|Viewport|AddtoViewport _returnvalue 0)
      (Variables|Default|SetHUD _returnvalue))
    (:then_1
      (CallFunction|CreateDynamicMaterial)
      (Default|UpdateCounterText (Variables|Default|GetHUD)))
    (:then_2
      (bind _returnvalue_2 (Actor|GetActorOfClass "/Game/Blueprints/BP_GenerateBananas.BP_GenerateBananas_C"))
      (Variables|Default|SetBananaGenerator _returnvalue_2)
      (Variables|Default|SetBananaFirstCount (Variables|/Game/Blueprints/BP_GenerateBananas.BP_GenerateBananas_C|GetCount (Variables|Default|GetBananaGenerator))))))

(event Input|AxisEvents|InputAxisMoveRight
  (params (AxisValue :type Float%20%28single-precision%29))
  (bind _returnvalue (Utilities|Time|GetWorldDeltaSeconds))
  ;[1 1 1] Moving
  (Transformation|AddActorWorldOffset (Math|Vector|MakeVector (* (stale Input|AxisEvents|InputAxisMoveForward AxisValue) (Variables|Default|GetspeedForward) _returnvalue) (* AxisValue (Variables|Default|GetspeedRight) _returnvalue) 0.0) true))

(event Input|AxisEvents|InputAxisMoveForward
  (params (AxisValue :type Float%20%28single-precision%29))
  ;[1 1 1] Moving
)

(fn ConstructionScript)

(fn CreateDynamicMaterial
  (bind _returnvalue (Rendering|Material|CreateDynamicMaterialInstance (Variables|Default|GetStaticMesh) 0 "/Game/Materials/M_Cube.M_Cube" "None" :!class /Script/Engine.PrimitiveComponent))
  (Variables|Default|SetCubeMaterial _returnvalue))