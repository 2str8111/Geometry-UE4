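; BP_Banana is a spinning banana actor that registers itself with the level's banana generator.
; On BeginPlay it finds the BP_GenerateBananas actor, caches it, and increments that generator's Count.
; Tick yaws the static mesh locally by Speed scaled by delta time, giving a frame-rate independent spin.
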(event EventBeginPlay
  (bind _returnvalue (Actor|GetActorOfClass "/Game/Blueprints/BP_GenerateBananas.BP_GenerateBananas_C"))
  (Variables|Default|SetBananaGenerator _returnvalue)
  (CallFunction|IncCount))

(event EventTick
  (params (DeltaSeconds :type Float%20%28single-precision%29))
  (Transformation|AddLocalRotation (Variables|Default|GetStaticMesh) (Math|Rotator|MakeRotator 0.0 0.0 (* DeltaSeconds (Variables|Default|Getspeed))) false false))

(fn ConstructionScript)

(fn IncCount
  (Math|Integer|IncrementInt (Variables|/Game/Blueprints/BP_GenerateBananas.BP_GenerateBananas_C|GetCount (Variables|Default|GetBananaGenerator))))