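; BP_GenerateBananas is an actor that fills an area with BP_Banana actors in a flat grid when play begins.
; BeginPlay calls GenerateBanana, which runs nested loops over the X and Y counts and spawns one banana per cell.
; Each position is offset from the actor's root world location by the cell index times Size, at the root's height.
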(event EventBeginPlay
  (CallFunction|GenerateBanana))

(fn ConstructionScript)

(fn GenerateBanana
  (bind _defaultsceneroot (Variables|Default|GetDefaultSceneRoot))
  (bind _returnvalue (Transformation|GetWorldLocation _defaultsceneroot))
  (for _index (range 0 (+ (Variables|Default|Getx) -1))
    (for _index_2 (range 0 (+ (Variables|Default|Gety) -1))
      (Game|SpawnActorfromClass "/Game/Blueprints/BP_Banana.BP_Banana_C" (Math|Transform|MakeTransform (Math|Vector|MakeVector (+ (* (Math|Conversions|ToFloat(Integer) _index) (Variables|Default|Getsize)) (.x _returnvalue)) (+ (.y _returnvalue) (* (Math|Conversions|ToFloat(Integer) _index_2) (Variables|Default|Getsize))) (.z _returnvalue)) "0, 0, 0" "1,1,1") "Undefined" 0 0))))